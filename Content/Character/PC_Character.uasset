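; Player character for a side-view rhythm platformer, moving and dashing in the Y-Z plane.
; Dash fires only within GM_rhythm's Tempo windows, line-traces to stop short of obstacles, then moves by timeline and swept Tick updates with gravity suspended.
; BeginPlay and checkpoints store respawn transforms in GM_rhythm, which respawns the character when destroyed.
; RythmAction pulses a scale indicator; debug keys change tempo or respawn at preset spots.
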(event OnComponentBeginOverlap(CapsuleComponent)
  (params (OverlappedComponent :type Primitive%20Component%20Object%20Reference) (OtherActor :type Actor%20Object%20Reference) (OtherComp :type Primitive%20Component%20Object%20Reference) (OtherBodyIndex :type Integer) (bFromSweep :type Boolean) (SweepResult :type Hit%20Result%20Structure%20%28by%20ref%29))
  (if (== (Utilities|GetClass OtherActor) "/Game/Blueprints/BP_checkpoint.BP_checkpoint_C")
    (bind _asgm_rhythm (Utilities|Casting|CastToGM_rhythm (Game|GetGameMode)))
    (Variables|/Game/Blueprints/GM_rhythm.GM_rhythm_C|SetRespawn%20Transform _asgm_rhythm (Transformation|GetActorTransform))))

(event Custom|Update%20anim
  (Sprite|SetFlipbook (Variables|Default|GetSprite) (select (> (Math|Vector|VectorLength (Variables|/Script/Engine.MovementComponent|GetVelocity (Variables|Character|GetCharacterMovement))) 0.0) "/Game/Test_Content/PNG/sprites/player/run/FB_Run.FB_Run" "/Game/Test_Content/PNG/sprites/player/idle/FB_Player_Idle.FB_Player_Idle")))

(event Custom|Update%20rotation
  (Math|Float|CompareFloat (.Y (Math|Vector|BreakVector (Variables|/Script/Engine.MovementComponent|GetVelocity (Variables|Character|GetCharacterMovement)))) 0.0
    (:>
      (Pawn|SetControlRotation (Pawn|GetController) (Math|Rotator|MakeRotator 0.0 0.0 9e+01)))
    (:<
      (Pawn|SetControlRotation (Pawn|GetController) (Math|Rotator|MakeRotator 0.0 0.0 -9e+01)))))

(event Custom|Exec%20dash
  (params (EndPosition :type Vector))
  (bind _newtrack_1 (Timeline|Dash PlayFromStart)
    (:Update
      (Variables|Default|SetNewVar (Math|Vector|Lerp(Vector) (Variables|Default|GetDashLocation) EndPosition _newtrack_1)))
    (:Finished
      (Variables|Default|SetisDashing false)
      (Components|Movement|StopMovementImmediately (Variables|Character|GetCharacterMovement)))))

(event Input|EnhancedActionEvents|EnhancedInputActionIA_Move
  (params (ActionValue :type Vector%202D%20Structure) (ElapsedSeconds :type Float%20%28double-precision%29) (TriggeredSeconds :type Float%20%28double-precision%29) (InputAction :type Input%20Action%20Object%20Reference :default "/Game/Blueprints/Inputs/IA_Move.IA_Move"))
  (if (not (Variables|Default|GetisDashing))
    (Pawn|Input|AddMovementInput "0.000000,1.000000,0.000000" (.x ActionValue) false)
    (Pawn|Input|AddMovementInput "0.000000,0.000000,1.000000" (.y ActionValue) false)
    (Variables|Default|SetForce%20Location (Math|Vector|MakeVector 0.0 (.x ActionValue) (.y ActionValue)))))

(event Input|EnhancedActionEvents|EnhancedInputActionIA_Dash
  (params (ActionValue :type Boolean) (ElapsedSeconds :type Float%20%28double-precision%29) (TriggeredSeconds :type Float%20%28double-precision%29) (InputAction :type Input%20Action%20Object%20Reference :default "/Game/Blueprints/Inputs/IA_Dash.IA_Dash"))
  (bind _returnvalue (Transformation|GetActorLocation))
  (bind _force_location (Variables|Default|GetForce%20Location))
  (bind _asgm_rhythm (Utilities|Casting|CastToGM_rhythm (Game|GetGameMode)))
  (if (>= (Variables|/Game/Blueprints/GM_rhythm.GM_rhythm_C|GetTempo _asgm_rhythm) 0.4)
    (Variables|Default|SetisDashing true :!label _label)
    (Variables|/Script/Engine.CharacterMovementComponent|SetGravityScale (Variables|Character|GetCharacterMovement) 0.0)
    (if (Utilities|Operators|NotEqual(!=) :A _force_location)
      (Variables|Default|SetDashEnd (+ (* _force_location 8e+01) (Transformation|GetActorLocation)))
      (Variables|Default|SetDashLocation _returnvalue)
      (bind _outhit (Collision|LineTraceByChannel _returnvalue (Variables|Default|GetDashEnd) "TraceTypeQuery1" false 0 "None"))
      (if (.bBlockingHit (Collision|BreakHitResult _outhit))
        (Variables|Default|SetImpact%20Point (.ImpactPoint (Collision|BreakHitResult _outhit)))
        (bind _offset (CallFunction|MakeOffset))
        (CallFunction|ExecDash _offset)
        (else
          (CallFunction|ExecDash (Variables|Default|GetDashEnd))))
      (else
        (Utilities|FlowControl|Delay 0.4)
        (Variables|Default|SetisDashing false)))
    (elif (<= (Variables|/Game/Blueprints/GM_rhythm.GM_rhythm_C|GetTempo _asgm_rhythm) 0.1)
      (goto _label))))

(event EventBeginPlay
  (Utilities|FlowControl|Sequence
    (:then_0
      (bind _returnvalue (Actor|GetActorOfClass "/Game/Blueprints/BP_CameraSpline.BP_CameraSpline_C"))
      (Variables|Default|SetCameraSpline _returnvalue)
      (bind _asplayer_controller (Utilities|Casting|CastToPlayerController (Pawn|GetController)))
      (Utilities|IsValid (PlayerController|LocalPlayerSubsystems|GetEnhancedInputLocalPlayerSubsystem _asplayer_controller)
        (:Is%20Valid
          (Input|AddMappingContext (PlayerController|LocalPlayerSubsystems|GetEnhancedInputLocalPlayerSubsystem _asplayer_controller) "/Game/Blueprints/Inputs/NewInputMappingContext.NewInputMappingContext" 0 "(bIgnoreAllPressedKeysUntilRelease=True,bForceImmediately=False,bNotifyUserSettings=False)")
          (bind _asgm_rhythm (Utilities|Casting|CastToGM_rhythm (Game|GetGameMode)))
          (Variables|/Game/Blueprints/GM_rhythm.GM_rhythm_C|SetRespawn%20Transform _asgm_rhythm (Transformation|GetActorTransform)))))
    (:then_1
      (Utilities|AsyncLoadAsset "/Game/StarterContent/Audio/Dash_.Dash_"))))

(event EventDestroyed
  (bind _asgm_rhythm (Utilities|Casting|CastToGM_rhythm (Game|GetGameMode)))
  (Default|RespawnPlayer _asgm_rhythm self))

(event EventRythmAction
  (bind _rythm (Variables|Default|Getrythm))
  (bind _newtrack_0 (Timeline|Timeline_0 PlayFromStart)
    (:Update
      (Transformation|SetRelativeScale3D _rythm (Math|Vector|Lerp(Vector) (Variables|Default|GetNull) (Variables|Default|GetHair%20size) _newtrack_0)))
    (:Finished
      (Transformation|SetRelativeScale3D _rythm "0, 0, 0"))))

(event EventTick
  (params (DeltaSeconds :type Float%20%28single-precision%29))
  (Variables|Default|SetForce%20Location "0, 0, 0")
  (Utilities|FlowControl|Sequence
    (:then_0
      (if (Variables|Default|GetisDashing)
        (Transformation|SetActorLocation (Variables|Default|GetNewVar) true true)))
    (:then_1
      (if (Variables|Default|GetisDashing)
        (Utilities|FlowControl|RetriggerableDelay 0.2)
        (bind _newtrack_0 (Timeline|gravity PlayFromStart)
          (:Update
            (Variables|/Script/Engine.CharacterMovementComponent|SetGravityScale (Variables|Character|GetCharacterMovement) (Math|Float|Lerp 0.0 5.0 _newtrack_0))))
        (else
          (Timeline|gravity Stop))))))

(event EventKill
  (Actor|DestroyActor))

(event Input|KeyboardEvents|DebugKeyEquals
  (params (Key :type Key%20Structure :default "None") (ActionValue :type Input%20Action%20Value%20Structure))
  (:Pressed
    (bind _returnvalue (Actor|GetActorOfClass "/Game/Blueprints/GM_rhythm.GM_rhythm_C"))
    (Default|AccelerateTempo _returnvalue)))

(event Input|KeyboardEvents|DebugKeyNumPadFour
  (params (Key :type Key%20Structure :default "None") (ActionValue :type Input%20Action%20Value%20Structure))
  (:Pressed
    (bind _asgm_rhythm (Utilities|Casting|CastToGM_rhythm (Game|GetGameMode)))
    (Variables|/Game/Blueprints/GM_rhythm.GM_rhythm_C|SetRespawn%20Transform _asgm_rhythm (Math|Transform|MakeTransform "1110.000000,-407.000000,388.000000" "0.000000,90.000000,0.000000" "1.000000,1.000000,1.000000"))
    (Actor|DestroyActor)))

(event Input|KeyboardEvents|DebugKeyNumPadFive
  (params (Key :type Key%20Structure :default "None") (ActionValue :type Input%20Action%20Value%20Structure))
  (:Pressed
    (bind _asgm_rhythm (Utilities|Casting|CastToGM_rhythm (Game|GetGameMode)))
    (Variables|/Game/Blueprints/GM_rhythm.GM_rhythm_C|SetRespawn%20Transform _asgm_rhythm (Math|Transform|MakeTransform "1110.000000,163.000000,103.000000" "0.000000,90.000000,0.000000" "1.000000,1.000000,1.000000"))
    (Actor|DestroyActor)))

(event Input|KeyboardEvents|DebugKeyNumPadSix
  (params (Key :type Key%20Structure :default "None") (ActionValue :type Input%20Action%20Value%20Structure))
  (:Pressed
    (bind _asgm_rhythm (Utilities|Casting|CastToGM_rhythm (Game|GetGameMode)))
    (Variables|/Game/Blueprints/GM_rhythm.GM_rhythm_C|SetRespawn%20Transform _asgm_rhythm (Math|Transform|MakeTransform "1110.000000,163.000000,388.000000" "0.000000,90.000000,0.000000" "1.000000,1.000000,1.000000"))
    (Actor|DestroyActor)))

(event Input|KeyboardEvents|DebugKeyNumPadOne
  (params (Key :type Key%20Structure :default "None") (ActionValue :type Input%20Action%20Value%20Structure))
  (:Pressed
    (bind _asgm_rhythm (Utilities|Casting|CastToGM_rhythm (Game|GetGameMode)))
    (Variables|/Game/Blueprints/GM_rhythm.GM_rhythm_C|SetRespawn%20Transform _asgm_rhythm (Math|Transform|MakeTransform "1110.000000,-1494.000000,103.000000" "0.000000,90.000000,0.000000" "1.000000,1.000000,1.000000"))
    (Actor|DestroyActor)))

(event Input|KeyboardEvents|DebugKeyRightParantheses
  (params (Key :type Key%20Structure :default "None") (ActionValue :type Input%20Action%20Value%20Structure))
  (:Pressed
    (bind _returnvalue (Actor|GetActorOfClass "/Game/Blueprints/GM_rhythm.GM_rhythm_C"))
    (Default|DecelerateTempo _returnvalue)))

(event Input|KeyboardEvents|DebugKeyNumPadTwo
  (params (Key :type Key%20Structure :default "None") (ActionValue :type Input%20Action%20Value%20Structure))
  (:Pressed
    (bind _asgm_rhythm (Utilities|Casting|CastToGM_rhythm (Game|GetGameMode)))
    (Variables|/Game/Blueprints/GM_rhythm.GM_rhythm_C|SetRespawn%20Transform _asgm_rhythm (Math|Transform|MakeTransform "1110.000000,-952.000000,103.000000" "0.000000,90.000000,0.000000" "1.000000,1.000000,1.000000"))
    (Actor|DestroyActor)))

(event Input|KeyboardEvents|DebugKeyNumPadThree
  (params (Key :type Key%20Structure :default "None") (ActionValue :type Input%20Action%20Value%20Structure))
  (:Pressed
    (bind _asgm_rhythm (Utilities|Casting|CastToGM_rhythm (Game|GetGameMode)))
    (Variables|/Game/Blueprints/GM_rhythm.GM_rhythm_C|SetRespawn%20Transform _asgm_rhythm (Math|Transform|MakeTransform "1110.000000,-407.000000,103.000000" "0.000000,90.000000,0.000000" "1.000000,1.000000,1.000000"))
    (Actor|DestroyActor)))

(fn ConstructionScript)

(fn MakeOffset
  (if (> (.y (Variables|Default|GetForce%20Location)) 0.0)
    (Variables|Default|SetImpact%20Point (Math|Vector|MakeVector (.x (Variables|Default|GetImpact%20Point)) (- (.y (Variables|Default|GetImpact%20Point)) 1e+01) (.z (Variables|Default|GetImpact%20Point)))))
  (if (< (.y (Variables|Default|GetForce%20Location)) 0.0)
    (Variables|Default|SetImpact%20Point (Math|Vector|MakeVector (.x (Variables|Default|GetImpact%20Point)) (+ (.y (Variables|Default|GetImpact%20Point)) 1e+01) (.z (Variables|Default|GetImpact%20Point)))))
  (if (> (.z (Variables|Default|GetForce%20Location)) 0.0)
    (Variables|Default|SetImpact%20Point (Math|Vector|MakeVector (.x (Variables|Default|GetImpact%20Point)) (.y (Variables|Default|GetImpact%20Point)) (- (.z (Variables|Default|GetImpact%20Point)) 1e+01))))
  (if (< (.z (Variables|Default|GetForce%20Location)) 0.0)
    (bind _output_get (Variables|Default|SetImpact%20Point (Math|Vector|MakeVector (.x (Variables|Default|GetImpact%20Point)) (.y (Variables|Default|GetImpact%20Point)) (+ (.z (Variables|Default|GetImpact%20Point)) 1e+01)))))
  (return _output_get))