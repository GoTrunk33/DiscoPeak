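; Rhythm game mode that keeps the beat, shows the W_Beats widget and handles player respawn.
; Tick accumulates time and, every 60/TempoMax seconds, calls RythmAction on the PC_Character and all BP_laserGun and BP_GroveBloc actors, found by class lookup on each beat.
; Debug events nudge TempoMax (BPM) up or down.
; RespawnPlayer spawns the player's class at RespawnTransform, possesses it and sets the view target to Camera.
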(event `/Game/Blueprints/BPI/BPI_Decelerate.Decelerate Tempo`
  ;[1 1 1] Debug rythm speed
  (bind _output_get (set `self.Tempo max` (- (`self.Tempo max`) 5.0)))
  (`KismetSystemLibrary.PrintString` (`KismetStringLibrary.Conv_DoubleToString` _output_get)))

(event `/Game/Blueprints/BPI/BPI_Accelerate.Accelerate Tempo`
  ;[1 1 1] Debug rythm speed
  (bind _output_get (set `self.Tempo max` (+ (`self.Tempo max`) 5.0)))
  (`KismetSystemLibrary.PrintString` (`KismetStringLibrary.Conv_DoubleToString` _output_get)))

(event `self.ReceiveBeginPlay`
  (set `self.Tempo` 0.15)
  (bind _returnvalue (`|CreateWidget` "/Game/UI/W_Beats.W_Beats_C"))
  (`UserWidget.AddToViewport` _returnvalue 0))

(event `self.ReceiveTick`
  (params (DeltaSeconds :type "Float (single-precision)"))
  (bind _returnvalue (/ 60.0 (`self.Tempo max`)))
  ;[1 1 1] Track rythm
  (set `self.Tempo` (+ (`self.Tempo`) DeltaSeconds))
  (if (>= (`self.Tempo`) _returnvalue)
    (set `self.Tempo` (- (`self.Tempo`) _returnvalue))
    ;[1 1 1] Send action to every bp
    (bind _returnvalue_2 (`GameplayStatics.GetActorOfClass` "/Game/Character/PC_Character.PC_Character_C"))
    (`/Game/Blueprints/BPI/BPI_Rythm.Rythm action` _returnvalue_2)
    (bind _outactors (`GameplayStatics.GetAllActorsOfClass` "/Game/Blueprints/Traps/BP_laserGun.BP_laserGun_C"))
    (for _array_element _outactors
      (`/Game/Blueprints/BPI/BPI_Rythm.Rythm action` _array_element))
    (bind _outactors_2 (`GameplayStatics.GetAllActorsOfClass` "/Game/Blueprints/Traps/BP_GroveBloc.BP_GroveBloc_C"))
    (for _array_element_2 _outactors_2
      (`/Game/Blueprints/BPI/BPI_Rythm.Rythm action` _array_element_2))))

(event `Respawn Player`
  (params (Player :type "/Game/Character/PC_Character Object Reference"))
  (bind _returnvalue (`GameplayStatics.GetPlayerController` 0))
  (bind _returnvalue_2 (`|SpawnActorFromClass` (`GameplayStatics.GetObjectClass` Player) (`self.Respawn Transform`) "Undefined" "MultiplyWithRoot" null null))
  (`Controller.Possess` _returnvalue _returnvalue_2)
  (`PlayerController.SetViewTargetWithBlend` _returnvalue (`self.Camera`) 0.0 "VTBlend_Linear" 0.0 false))

(fn `UserConstructionScript`)