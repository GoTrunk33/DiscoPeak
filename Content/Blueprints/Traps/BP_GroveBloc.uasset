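; BP_GroveBloc is a trap block that moves back and forth between its start position and an AddPos offset in rhythm.
; RythmAction counts beats and, every NumberOfBeats, a FlipFlop alternates between two timelines.
; Each timeline lerps from the current location toward its endpoint without sweeping, so the motion eases rather than following the curve directly.
; The Grove hit event is empty; logic to kill PC_Character is left disconnected.
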(event `self.ReceiveBeginPlay`
  (bind _returnvalue (`self.K2_GetActorLocation`))
  (set `self.Pos0` _returnvalue)
  (set `self.Pos1` (+ _returnvalue (`self.Add_pos`))))

(event `/Game/Blueprints/BPI/BPI_Rythm.Rythm action`
  (bind _result (`/Engine/EditorBlueprintResources/StandardMacros.IncrementInt` (`self.Beats count`))
    (:`  `
      (if (== _result (`self.Number of beats`))
        (set `self.Beats count` 0)
        (`/Engine/EditorBlueprintResources/StandardMacros.FlipFlop`
          (:`A`
            (bind (_direction _movement) (`Timeline|Timeline` :!via `PlayFromStart`)
              (:`Update`
                (`self.K2_SetActorLocation` (`KismetMathLibrary.VLerp` (`self.K2_GetActorLocation`) (`self.Pos1`) _movement)))))
          (:`B`
            (bind (_direction_2 _movement_2) (`Timeline|Timeline_0` :!via `PlayFromStart`)
              (:`Update`
                (`self.K2_SetActorLocation` (`KismetMathLibrary.VLerp` (`self.K2_GetActorLocation`) (`self.Pos0`) _movement_2))))))))))

(event `self.grove.OnComponentHit`
  (params (HitComponent :type "PrimitiveComponent Object Reference") (OtherActor :type "Actor Object Reference") (OtherComp :type "PrimitiveComponent Object Reference") (NormalImpulse :type "Vector Structure") (Hit :type "HitResult Structure (by ref)")))

(fn `UserConstructionScript`)