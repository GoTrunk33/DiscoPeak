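; Rhythm game mode that acts as the beat clock, showing the W_Beats widget and playing a 120 BPM metronome loop.
; Tick accumulates time and, on each TempoMax-derived beat, calls RythmAction on PC_Character and every BP_GroveBloc.
; Accelerate and decelerate events shift TempoMax without altering the audio loop.
; RespawnPlayer spawns a new instance of the player's class, possesses it and sets the view target to Camera.
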(event `/Game/Blueprints/BPI/BPI_Decelerate.Decelerate Tempo`
  (bind _output_get (set `self.Tempo max` (- (`self.Tempo max`) 5.0)))
  (`KismetSystemLibrary.PrintString` (`KismetStringLibrary.Conv_DoubleToString` _output_get)))

(event `/Game/Blueprints/BPI/BPI_Accelerate.Accelerate Tempo`
  (bind _output_get (set `self.Tempo max` (+ (`self.Tempo max`) 5.0)))
  (`KismetSystemLibrary.PrintString` (`KismetStringLibrary.Conv_DoubleToString` _output_get)))

(event `self.ReceiveBeginPlay`
  (bind _returnvalue (`|GenericCreateObject` "/Game/UI/W_Beats.W_Beats_C"))
  (`UserWidget.AddToViewport` _returnvalue 0)
  (`GameplayStatics.PlaySound2D` "/Game/Added/Disco_Drum_Metronome_Loop_120_BPM.Disco_Drum_Metronome_Loop_120_BPM" 1.0 1.0 0.0 null null))

(event `self.ReceiveTick`
  (params (DeltaSeconds :type "Float (single-precision)"))
  (bind _returnvalue (/ 60.0 (`self.Tempo max`)))
  (set `self.Tempo` (+ (`self.Tempo`) DeltaSeconds))
  (if (>= (`self.Tempo`) _returnvalue)
    (set `self.Tempo` (- (`self.Tempo`) _returnvalue))
    (bind _returnvalue_2 (`GameplayStatics.GetActorOfClass` "/Game/Character/PC_Character.PC_Character_C"))
    (`/Game/Blueprints/BPI/BPI_Rythm.Rythm action` _returnvalue_2)
    (bind _outactors (`GameplayStatics.GetAllActorsOfClass` "/Game/Blueprints/BP_GroveBloc.BP_GroveBloc_C"))
    (for _array_element _outactors
      (`/Game/Blueprints/BPI/BPI_Rythm.Rythm action` _array_element))))

(event `Respawn Player`
  (params (Player :type "/Game/Character/PC_Character Object Reference"))
  (bind _returnvalue (`GameplayStatics.GetPlayerController` 0))
  (`KismetSystemLibrary.PrintString` "Hello")
  (bind _returnvalue_2 (`|SpawnActorFromClass` (`GameplayStatics.GetObjectClass` Player) (`self.Respawn Transform`) "Undefined" "MultiplyWithRoot" null null))
  (`Controller.Possess` _returnvalue _returnvalue_2)
  (`PlayerController.SetViewTargetWithBlend` _returnvalue (`self.Camera`) 0.0 "VTBlend_Linear" 0.0 false))

(fn `UserConstructionScript`)