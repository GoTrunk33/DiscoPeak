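; BP_Bluedoor1 is a door mechanism that slides toward an open position when its Open event fires.
; Open raises the On flag for one second, then clears it.
; While On is set, Tick eases the actor toward EndPos with VInterpTo and no sweep, so movement stops when the timer ends, whether or not it has arrived.
; EndPos is not computed in these graphs.
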(event `self.Open`
  ;[1 1 1] Calculate open state coords
  (set `self.On` true)
  (`KismetSystemLibrary.Delay` 1.0)
  (set `self.On` false))

(event `self.ReceiveTick`
  (params (DeltaSeconds :type "Float (single-precision)"))
  ;[1 1 1] Open door when button is triggered
  (if (`self.On`)
    (`self.K2_SetActorLocation` (`KismetMathLibrary.VInterpTo` (`self.K2_GetActorLocation`) (`self.End_Pos`) (`GameplayStatics.GetWorldDeltaSeconds`) 2.0))))

(fn `UserConstructionScript`)