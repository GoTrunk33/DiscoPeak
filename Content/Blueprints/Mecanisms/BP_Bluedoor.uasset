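; BP_Bluedoor is a door mechanism that slides upward when its Open event is called.
; Open sets a target 100 units above the current location and enables movement for one second.
; While enabled, Tick eases the actor toward that target with VInterpTo, without sweeping.
; Movement stops on the timer rather than on arrival, and the file has no closing logic.
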(event `/Game/Blueprints/BPI/BPI_Door.Open`
  (set `self.End_Pos` (+ (`self.K2_GetActorLocation`) (0.0 0.0 100.0)))
  (set `self.On` true)
  (`KismetSystemLibrary.Delay` 1.0)
  (set `self.On` false))

(event `self.ReceiveTick`
  (params (DeltaSeconds :type "Float (single-precision)"))
  (if (`self.On`)
    (`self.K2_SetActorLocation` (`KismetMathLibrary.VInterpTo` (`self.K2_GetActorLocation`) (`self.End_Pos`) (`GameplayStatics.GetWorldDeltaSeconds`) 2.0))))

(fn `UserConstructionScript`)