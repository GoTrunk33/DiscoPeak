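; Rhythm-driven block actor that moves back and forth between its start location and an offset set by AddPos.
; Each RythmAction call counts a beat, and reaching NumberOfBeats flips the travel direction through a FlipFlop and plays that direction's timeline.
; The timelines lerp from the current location rather than a fixed start, and the beat count resets only when the move finishes.
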(event `self.ReceiveBeginPlay`
  (bind _returnvalue (`self.K2_GetActorLocation`))
  (set `self.Pos0` _returnvalue)
  (set `self.Pos1` (+ _returnvalue (`self.Add_pos`))))

(event `/Game/Blueprints/BPI/BPI_Rythm.Rythm action`
  (bind _result (`/Engine/EditorBlueprintResources/StandardMacros.IncrementInt` (`self.Beats count`))
    (:`  `
      (if (== _result (`self.Number of beats`))
        (`/Engine/EditorBlueprintResources/StandardMacros.FlipFlop`
          (:`A`
            (bind (_direction _newtrack_0) (`Timeline|Timeline` :!via `PlayFromStart`)
              (:`Update`
                (`self.K2_SetActorLocation` (`KismetMathLibrary.VLerp` (`self.K2_GetActorLocation`) (`self.Pos1`) _newtrack_0)))
              (:`Finished`
                (set `self.Beats count` 0))))
          (:`B`
            (bind (_direction_2 _newtrack_0_2) (`Timeline|Timeline_0` :!via `PlayFromStart`)
              (:`Update`
                (`self.K2_SetActorLocation` (`KismetMathLibrary.VLerp` (`self.K2_GetActorLocation`) (`self.Pos0`) _newtrack_0_2)))
              (:`Finished`
                (set `self.Beats count` 0)))))))))

(fn `UserConstructionScript`)